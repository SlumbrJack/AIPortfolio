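; Enemy AI controller that turns sight perception of the player into Blackboard data.
; Perception info updates pass the target and stimulus to HandleSightSense, which ignores other senses and any actor except player character 0.
; A successful sighting stores the player as TargetActor; losing sight clears that key and records the stimulus position as LastKnownLocation.
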(event `self.yomamadeez.OnTargetPerceptionInfoUpdated`
  (params (UpdateInfo :type "ActorPerceptionUpdateInfo Structure (by ref)"))
  (`self.HandleSightSense` UpdateInfo_Target UpdateInfo_Stimulus))

(event `self.yomamadeez.OnTargetPerceptionUpdated`
  (params (Actor :type "Actor Object Reference") (Stimulus :type "AIStimulus Structure")))

(fn `HandleSightSense`
  (params (Actor :type "Actor Object Reference") (Stimulu :type "AIStimulus Structure"))
  (bind (_stimulu_age _stimulu_expirationage _stimulu_strength _stimulu_stimuluslocation _stimulu_receiverlocation _stimulu_tag _stimulu_bsuccessfullysensed) (break `AIStimulus` (`local.Stimulu`)))
  (bind _returnvalue (`AIPerceptionSystem.GetSenseClassForStimulus` Stimulu))
  (if (== _returnvalue "/Script/AIModule.AISense_Sight")
    (if (== (`GameplayStatics.GetPlayerCharacter` 0) (`local.Actor`))
      (`BlackboardComponent.SetValueAsObject` (`AIBlueprintHelperLibrary.GetBlackboard` null) "TargetActor" (`KismetMathLibrary.SelectObject` (`GameplayStatics.GetPlayerCharacter` 0) null _stimulu_bsuccessfullysensed))
      (if (not _stimulu_bsuccessfullysensed)
        (`BlackboardComponent.SetValueAsVector` (`AIBlueprintHelperLibrary.GetBlackboard` null) "LastKnownLocation" _stimulu_stimuluslocation))
      (else
        (return)))
    (else
      (return))))

(fn `UserConstructionScript`)